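; BP_AntEnemy is an ant enemy that chases the player once it spots a pawn.
; Tick halts movement until PawnSensing fires, then AIMoveTo heads for the player and plays an attack montage on arrival.
; Body collision overlap applies damage to girl_bp, independent of the montage.
; TakeDamage removes one health per call and destroys the ant at zero, with Die left empty.
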(event OnSeePawn(PawnSensing)
  (params (Pawn :type Pawn%20Object%20Reference))
  (Variables|Default|SetIsSeePlayer? true)
  (CallFunction|FollowPlayer))

(event OnComponentBeginOverlap(Body_collision)
  (params (OverlappedComponent :type Primitive%20Component%20Object%20Reference) (OtherActor :type Actor%20Object%20Reference) (OtherComp :type Primitive%20Component%20Object%20Reference) (OtherBodyIndex :type Integer) (bFromSweep :type Boolean) (SweepResult :type Hit%20Result%20Structure%20%28by%20ref%29))
  (bind _asgirl_bp (Utilities|Casting|CastTogirl_bp OtherActor))
  (Game|Damage|ApplyDamage _asgirl_bp 5.0 0 0))

(event Custom|FollowPlayer
  (Variables|Default|SetCanAttack? true)
  (if (Variables|Default|GetIsSeePlayer?)
    (AI|AIMoveTo self "0, 0, 0" (Game|GetPlayerCharacter 0) 7e+01 false
      (:OnSuccess
        (Variables|Default|SetCanAttack? (Variables|Default|GetCanAttack?))
        (if true
          (Animation|PlayAnimMontage "/Game/Enemy/ANT/Animation/AM_Ant_Attack.AM_Ant_Attack" 1.0 "None")
          (Utilities|FlowControl|Delay 0.2)
          (Variables|Default|SetCanAttack? true)
          (else
            (Variables|Default|SetIsSeePlayer? false)))))))

(event Custom|TakeDamage
  (bind _output_get (Variables|Default|Sethealth (- (Variables|Default|Gethealth) 1)))
  (if (<= _output_get 0)
    (CallFunction|Die)
    (Actor|DestroyActor)))

(event Custom|Die)

(event EventBeginPlay)

(event Collision|EventActorBeginOverlap
  (params (OtherActor :type Actor%20Object%20Reference)))

(event EventTick
  (params (DeltaSeconds :type Float%20%28single-precision%29))
  (if (not (Variables|Default|GetIsSeePlayer?))
    (Components|Movement|StopMovementImmediately (Variables|Character|GetCharacterMovement))))

(fn ConstructionScript)